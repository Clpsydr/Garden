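; Laser death trap for the PhysTrial area, switched on or off by whether something blocks a short upward trace from its activation device, with an option to reverse the logic.
; Tick runs that trace and toggles the three laser components.
; While active, a looping timer box-traces between two cone components and applies damage with a knockback impulse to any player pawn hit.
; Debug trace drawing and hit-name printing remain enabled.
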(event `self.ReceiveBeginPlay`
  (`KismetSystemLibrary.K2_SetTimerDelegate` (delegate `UseLaser`) (`self.CheckFreq`) true))

(event `UseLaser`
  ;[1 1 1] Laser killcheck
  (if (`self.bActivated`)
    (bind _outhit (`KismetSystemLibrary.BoxTraceSingleByProfile` :`Start` (`SceneComponent.K2_GetComponentLocation` (`self.OutCone2`)) :`End` (`SceneComponent.K2_GetComponentLocation` (`self.InCone2`)) :`HalfSize` (5.0 0.0 80.0) :`ProfileName` "PlayerAllies" :`DrawDebugType` "Persistent" :`TraceColor` (struct :`G` 0.075142 :`B` 1.0 :`A` 1.0) :`DrawTime` 0.2))
    (if (`GameplayStatics.BreakHitResult` _outhit)
      (`KismetSystemLibrary.PrintString` (`KismetSystemLibrary.GetObjectName` (`.HitActor` (`GameplayStatics.BreakHitResult` _outhit))))
      (bind _asbp_player_pawn (cast `/Game/Blueprints/BP_PlayerPawn` (`.HitActor` (`GameplayStatics.BreakHitResult` _outhit))))
      (`/Game/Blueprints/BP_PlayerPawn.BoneitisDmg` _asbp_player_pawn 60.0 (* (`.ImpactNormal` (`GameplayStatics.BreakHitResult` _outhit)) 500.0) (`.Location` (`GameplayStatics.BreakHitResult` _outhit))))))

(event `self.ReceiveTick`
  (params (DeltaSeconds :type "Float (single-precision)"))
  (bind _returnvalue (`SceneComponent.K2_GetComponentLocation` (`self.ActivationDevice`)))
  ;[1 1 1] Switch control
  (bind (_outhit _returnvalue_2) (`KismetSystemLibrary.LineTraceSingle` :`Start` (+ _returnvalue (0.0 0.0 1.0)) :`End` (+ _returnvalue (0.0 0.0 50.0)) :`TraceChannel` "TraceTypeQuery1" :`DrawDebugType` "Persistent"))
  (if (xor (`self.ReverseActivation`) _returnvalue_2)
    (if (not (`self.bActivated`))
      (set `self.bActivated` true)
      (`ActorComponent.Activate` (`self.Lasor2`) true)
      (`ActorComponent.Activate` (`self.Lasor3`) true)
      (`ActorComponent.Activate` (`self.Lasor1`) true))
    (else
      (set `self.bActivated` false)
      (`ActorComponent.Deactivate` (`self.Lasor1`))
      (`ActorComponent.Deactivate` (`self.Lasor2`))
      (`ActorComponent.Deactivate` (`self.Lasor3`)))))

(fn `UserConstructionScript`)
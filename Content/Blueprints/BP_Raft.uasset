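; BP_Raft is a raft that the player can board and take control of.
; InteractTouch has the interacting player's BP_PlayerController switch its pawn to the raft, then calls Piloted(true).
; Piloted shows or hides the SkeletalMesh and its children to match the piloted state.
; A Sphere overlap only prints a debug message when a BP_PlayerPawn comes close.
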(event `self.ReceiveBeginPlay`)

(event `self.Sphere.OnComponentBeginOverlap`
  (params (OverlappedComponent :type "PrimitiveComponent Object Reference") (OtherActor :type "Actor Object Reference") (OtherComp :type "PrimitiveComponent Object Reference") (OtherBodyIndex :type Integer) (bFromSweep :type Boolean) (SweepResult :type "HitResult Structure (by ref)"))
  (cast `/Game/Blueprints/BP_PlayerPawn` OtherActor)
  (`KismetSystemLibrary.PrintString` "Close to player"))

(event `/Game/Blueprints/PhysTrial/BPI_BowlingInteraction.InteractTouch`
  (params (Player :type "/Game/Blueprints/BP_PlayerPawn Object Reference"))
  (bind _asbp_player_controller (cast `/Game/Blueprints/BP_PlayerController` (`self.GetController` Player)))
  (`MainPlayerController.ChangePawnTo` _asbp_player_controller self)
  (`self.Piloted` true))

(fn `Piloted`
  (params (bIsPiloted :type Boolean))
  (`SceneComponent.SetVisibility` (`self.SkeletalMesh`) bIsPiloted true))

(fn `UserConstructionScript`)
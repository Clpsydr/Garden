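; Player character pawn that fires bullets from its grab point along camera rotation, reports its controller's base HQ and toggles a weather particle effect.
; Capsule overlaps and hits pass the player to BPI_PlayerInteraction actors to apply their effects, destroying overlapped ones.
; BoneitisDmg lowers HP and, at zero, ragdolls the mesh, breaks spine, neck and pelvis constraints and disables movement.
; Physical animation blending is experimental; unpossessed pawns soon expire.
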(event `self.ReceiveTick`
  (params (DeltaSeconds :type "Float (single-precision)")))

(event `self.ReceiveBeginPlay`
  (bind _in_bone_name (`self.In Bone Name`))
  (bind _physicalanimation (`self.PhysicalAnimation`))
  (bind _mesh (`self.Mesh`))
  ;[1 1 1] Blending ragdoll with skeletal animation (not working well with this skeleton)
  (`PhysicalAnimationComponent.SetSkeletalMeshComponent` _physicalanimation _mesh)
  (`PhysicalAnimationComponent.ApplyPhysicalAnimationProfileBelow` _physicalanimation _in_bone_name "DefaultProf" true false)
  (`SkeletalMeshComponent.SetAllBodiesBelowSimulatePhysics` _mesh _in_bone_name false true)
  (`PhysicalAnimationComponent.SetStrengthMultiplyer` _physicalanimation 5.0))

(event `self.CapsuleComponent.OnComponentBeginOverlap`
  (params (OverlappedComponent :type "PrimitiveComponent Object Reference") (OtherActor :type "Actor Object Reference") (OtherComp :type "PrimitiveComponent Object Reference") (OtherBodyIndex :type Integer) (bFromSweep :type Boolean) (SweepResult :type "HitResult Structure (by ref)"))
  ;[1 1 1] Energy pickup further extended to all pickups
  (if (`KismetSystemLibrary.DoesImplementInterface` OtherActor "/Game/Blueprints/PhysTrial/BPI_PlayerInteraction.BPI_PlayerInteraction_C")
    (message `/Game/Blueprints/PhysTrial/BPI_PlayerInteraction.ContextualPlayerEffect` OtherActor self (0.0 0.0 0.0) (0.0 0.0 0.0))
    (`self.K2_DestroyActor` OtherActor)))

(event `self.CapsuleComponent.OnComponentHit`
  (params (HitComponent :type "PrimitiveComponent Object Reference") (OtherActor :type "Actor Object Reference") (OtherComp :type "PrimitiveComponent Object Reference") (NormalImpulse :type "Vector Structure") (Hit :type "HitResult Structure (by ref)"))
  ;[1 1 1] if interactable object is hit, look up its effect on player
  (if (`KismetSystemLibrary.DoesImplementInterface` OtherActor "/Game/Blueprints/PhysTrial/BPI_PlayerInteraction.BPI_PlayerInteraction_C")
    (message `/Game/Blueprints/PhysTrial/BPI_PlayerInteraction.ContextualPlayerEffect` OtherActor self (* NormalImpulse 500.0) Hit_Location)))

(event `self.ReceiveUnpossessed`
  (params (OldController :type "Controller Object Reference"))
  ;[1 0.03704 0.2889 1 40] Pawn destroyed if not controlled
  (`self.SetLifeSpan` 0.3))

(fn `BoneitisDmg`
  (params (DamageAmount :type "Float (double-precision)") (HitImpulse :type "Vector Structure") (HitLocation :type "Vector Structure"))
  (bind _mesh (`self.Mesh`))
  (bind _output_get (set `self.CurrentHp` (- (`self.CurrentHp`) DamageAmount)))
  (`/Engine/EditorBlueprintResources/StandardMacros.CompareFloat` _output_get
    (:`==`
      _)
    (:`<`
      _))
  (`PrimitiveComponent.SetSimulatePhysics` _mesh true)
  (`SkeletalMeshComponent.BreakConstraint` _mesh HitImpulse HitLocation "neck_01")
  (`SkeletalMeshComponent.BreakConstraint` _mesh HitImpulse HitLocation "spine_01")
  (`SkeletalMeshComponent.BreakConstraint` _mesh HitImpulse HitLocation "spine_02")
  (`SkeletalMeshComponent.BreakConstraint` _mesh HitImpulse HitLocation "pelvis")
  (`CharacterMovementComponent.DisableMovement` (`self.CharacterMovement`)))

(fn `FireGun`
  (`|SpawnActorFromClass` "/Game/Blueprints/BP_BasicBullet.BP_BasicBullet_C" (`KismetMathLibrary.MakeTransform` (`SceneComponent.K2_GetComponentLocation` (`self.ItemGrabLocation`)) (`SceneComponent.K2_GetComponentRotation` (`self.Camera`))) "Undefined" "OverrideRootScale" null null))

(fn `ReturnBase`
  (returns (NewParam :type "HomeBase Object Reference"))
  (bind _asbp_player_controller (cast `/Game/Blueprints/BP_PlayerController` (`self.GetController`)))
  (return (`/Game/Blueprints/BP_PlayerController.BaseHQ` _asbp_player_controller)))

(fn `UserConstructionScript`)

(fn `WeatherActivate`
  (params (bTurnOn :type Boolean))
  (bind _shinyparticleeffect (`self.ShinyParticleEffect`))
  (if bTurnOn
    (`ActorComponent.Activate` _shinyparticleeffect false)
    (else
      (`ActorComponent.Deactivate` _shinyparticleeffect))))
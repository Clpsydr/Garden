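; Player controller that sets up the HUD, caches the HomeBase actor, and handles raft exit and map input.
; On Interact while piloting BP_Raft, it clears the piloted state, spawns a BP_PlayerPawn with a raised offset and switches control to it.
; A zoom axis adjusts the status window's minimap within clamped limits, while holding ShowFullMap swaps that window for a large map widget.
; Game-over camera logic exists but is unconnected.
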(event `self.ReceiveBeginPlay`
  ;[1 1 1] UI setup
  (`self.InitHUD`)
  ;[1 1 1] Locating Base
  (bind _returnvalue (`GameplayStatics.GetActorOfClass` "/Script/GardenTD.HomeBase"))
  (set `self.BaseHQ` _returnvalue))

(event `InputAction|Interact`
  (params (Key :type "Key Structure"))
  (:`Pressed`
    ;[0.2917 0.2917 0.2917 1 40] Deboating process
    (bind _asbp_raft (cast `/Game/Blueprints/BP_Raft` (`GameplayStatics.GetPlayerPawn` 0)))
    (`/Game/Blueprints/BP_Raft.Piloted` _asbp_raft false)
    (bind (_returnvalue_location _returnvalue_rotation _returnvalue_scale) (`KismetMathLibrary.BreakTransform` (`self.GetTransform` _asbp_raft)))
    (bind _returnvalue (`|SpawnActorFromClass` "/Game/Blueprints/BP_PlayerPawn.BP_PlayerPawn_C" (`KismetMathLibrary.MakeTransform` (+ (0.0 0.0 0.0) (0.0 0.0 200.0)) (struct) _returnvalue_scale) "AlwaysSpawn" "OverrideRootScale" null null))
    (`self.ChangePawnTo` _returnvalue)))

(event `self.ReceiveTick`
  (params (DeltaSeconds :type "Float (single-precision)")))

(event `InputAxis|MinimapZoom`
  (params (AxisValue :type "Float (single-precision)"))
  ;[1 1 1] Map Zooming controls
  (`/Engine/EditorBlueprintResources/StandardMacros.CompareFloat` AxisValue
    (:`>`
      _)
    (:`<`
      _))
  (bind _returnvalue (`self.GetPlayerStatusWindow`))
  (bind _asbpui_player_status (cast `/Game/Blueprints/UI/BPUI_PlayerStatus` _returnvalue))
  (bind _bpui_minimap (`/Game/Blueprints/UI/BPUI_PlayerStatus.BPUI_Minimap` _asbpui_player_status))
  (set `/Game/Blueprints/UI/MapUI/BPUI_Minimap.Zoom` (`KismetMathLibrary.FClamp` (+ (`/Game/Blueprints/UI/MapUI/BPUI_Minimap.Zoom` _bpui_minimap) (* AxisValue -0.1)) 0.3 0.8) _bpui_minimap))

(event `InputAction|ShowFullMap`
  (params (Key :type "Key Structure"))
  ;[1 1 1] Map Fullscreen
  (:`Pressed`
    (bind _returnvalue (`|CreateWidget` "/Game/Blueprints/UI/MapUI/BPUI_LargeMap.BPUI_LargeMap_C"))
    (bind _output_get (set `self.MapUI` _returnvalue))
    (`UserWidget.AddToViewport` _output_get 0)
    (bind _returnvalue_2 (`self.GetPlayerStatusWindow`))
    (`Widget.SetVisibility` _returnvalue_2 "Hidden"))
  (:`Released`
    (bind _mapui (`self.MapUI`)
      (:`then`
        (`Widget.RemoveFromParent` _mapui)
        (`self.GetPlayerStatusWindow`)
        (`Widget.SetVisibility` _returnvalue_2 "Visible"))
      (:`else`))))

(fn `UserConstructionScript`)